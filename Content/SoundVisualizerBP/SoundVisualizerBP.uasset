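; Sound visualizer actor that animates instanced-mesh bars from FFT analysis of audio output.
; Construction script lays out bars as line, circle, grid or spline, adding instances for top pieces, mirrored bars or stacked steps.
; A 0.1-second timer turns frequency magnitudes into log-scaled target transforms.
; Once the first targets exist, gated Tick smooths instances toward them per movement mode (scale, location, both, or step), with slowly falling top pieces.
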(event `self.ReceiveBeginPlay`
  (`AudioMixerBlueprintLibrary.StartAnalyzingOutput` null "Max" :!label _label)
  (`KismetSystemLibrary.K2_SetTimerDelegate` (delegate `UpdataTransform`) 0.1 true))

(event `シーケンサー用`
  (goto _label))

(event `UpdataTransform`
  (bind _magnitudes (`AudioMixerBlueprintLibrary.GetMagnitudeForFrequencies` (`self.Frequency`) null))
  (`KismetArrayLibrary.Array_Clear` (`self.Tmp`))
  (for (_array_element _array_index) _magnitudes
    (bind _outinstancetransform (`InstancedStaticMeshComponent.GetInstanceTransform` (`self.Ber`) _array_index false))
    (bind _returnvalue (* (`KismetMathLibrary.Log` (`KismetMathLibrary.FMax` _array_element 1.0) 2.7) (`self.sensitivity`)))
    (bind _returnvalue_2 (`KismetMathLibrary.MakeTransform` (.location _outinstancetransform) (.rotation _outinstancetransform) (`KismetMathLibrary.MakeVector` (.x (.scale _outinstancetransform)) (.y (.scale _outinstancetransform)) _returnvalue)))
    (bind _transform (`self.ローテーションから向きを取得` (`self.BaseTransform`) _array_index _returnvalue))
    (`KismetArrayLibrary.Array_Add` (`self.Tmp`) (select `/Game/SoundVisualizerBP/Enum/BarMovement` (`self.Bar movement`) :`NewEnumerator0` _returnvalue_2 :`NewEnumerator1` _returnvalue_2 :`NewEnumerator2` _transform :`NewEnumerator3` _transform :`NewEnumerator4` _transform :`NewEnumerator5` _returnvalue_2)))
  (`/Engine/EditorBlueprintResources/StandardMacros.DoOnce` false
    (:`Completed`
      (`self.格納完了`))))

(event `self.ReceiveTick`
  (params (DeltaSeconds :type "Float (single-precision)"))
  (bind _top_one_bers (`self.Top one Bers`))
  (bind _number_of_bars (`self.Number of bars`))
  (bind _number_of_bars_2 (`self.Number of bars`))
  (bind _number_of_bars_3 (`self.Number of bars`))
  (bind _returnvalue (- 1.0 (`self.smooth`)))
  (bind _returnvalue_2 (* _number_of_bars_3 (`self.Division number`)))
  (bind _returnvalue_3 (select `bool` (== (`self.Bar movement`) 5) :`false` (select `bool` _top_one_bers :`false` _number_of_bars_3 :`true` (* _number_of_bars_3 2)) :`true` (select `bool` _top_one_bers :`false` _returnvalue_2 :`true` (+ _returnvalue_2 _number_of_bars_3))))
  (`/Engine/EditorBlueprintResources/StandardMacros.Gate` true :!label _label_2
    (:`Exit`
      (for _index (range (select `bool` (== (`self.Bar movement`) 4) :`false` _returnvalue_3 :`true` (* _returnvalue_3 2)))
        (if (== (`self.Bar movement`) 5)
          ;[1 1 1] ステップ更新
          (if (== (mod (+ _index 1) (`self.Number of bars`)) 0)
            (`|ExecutionSequence`
              (:`then_0`
                (bind _outinstancetransform (`InstancedStaticMeshComponent.GetInstanceTransform` (`self.Ber`) _index false))
                (bind _outinstancetransform_2 (`InstancedStaticMeshComponent.GetInstanceTransform` (`self.Ber`) _index false))
                (bind _returnvalue_4 (`KismetMathLibrary.FClamp` (`KismetMathLibrary.NormalizeToRange` (.z (.scale (`|GetArrayItem` (`self.Tmp`) (- _index (* (`self.Number of bars`) (`self.stepheight`)))))) 0.0 20.0)))
                (bind _returnvalue_5 (select `bool` (>= _returnvalue_4 (/ (`KismetMathLibrary.Conv_IntToDouble` (+ (`self.stepheight`) 1)) (`KismetMathLibrary.Conv_IntToDouble` (`self.Division number`)))) :`true` 1.0 :!type "Float (single-precision)"))
                (bind _returnvalue_6 (select `bool` (`self.interpolation`) :`false` _returnvalue_5 :`true` (`KismetMathLibrary.Lerp` (.z (.scale _outinstancetransform)) _returnvalue_5 (- 1.0 (`self.smooth`)))))
                (bind _returnvalue_7 (* (+ (`KismetMathLibrary.Conv_IntToDouble` (`self.Division number`)) -0.5) _returnvalue_4 (`self.Bar spacing`)))
                (`InstancedStaticMeshComponent.UpdateInstanceTransform` (`self.Ber`) _index (select `bool` (> _index (* (`self.Number of bars`) (`self.Division number`))) :`false` (`KismetMathLibrary.MakeTransform` (.location _outinstancetransform) (.rotation _outinstancetransform_2) (`KismetMathLibrary.MakeVector` _returnvalue_6 _returnvalue_6 _returnvalue_6)) :`true` (`KismetMathLibrary.MakeTransform` (`KismetMathLibrary.MakeVector` (.x (.location _outinstancetransform_2)) (.y (.location _outinstancetransform_2)) (select `bool` (>= (.z (.location _outinstancetransform_2)) _returnvalue_7) :`false` (`KismetMathLibrary.Lerp` (.z (.location _outinstancetransform_2)) _returnvalue_7 0.5) :`true` (`KismetMathLibrary.FInterpTo` (.z (.location _outinstancetransform_2)) 0.0 (`GameplayStatics.GetWorldDeltaSeconds`) 0.25))) (.rotation _outinstancetransform_2) (`self.top one scale`))) false true false :!label _label_3))
              (:`then_1`
                (`/Engine/EditorBlueprintResources/StandardMacros.IncrementInt` (`self.stepheight`))))
            (else
              (goto _label_3)))
          (else
            (bind _returnvalue_8 (select `bool` (> _index (- _number_of_bars_2 1)) :`false` _index :`true` (- _index _number_of_bars_2)))
            (bind _output (`|GetArrayItem` (`self.Tmp`) _returnvalue_8))
            (bind _returnvalue_9 (`KismetMathLibrary.MakeTransform` (.location _output) (.rotation _output) (`KismetMathLibrary.MakeVector` (.x (.scale _output)) (.y (.scale _output)) (`KismetMathLibrary.FMax` (`KismetMathLibrary.Lerp` (.z (.scale _outinstancetransform)) (.z (.scale _output)) (- 1.0 (`self.smooth`))) 0.001))))
            (bind _z (.z (.location _outinstancetransform)))
            (bind _returnvalue_10 (* (.z (.scale _output)) 92.0))
            (bind _returnvalue_11 (`KismetMathLibrary.MakeTransform` (`KismetMathLibrary.MakeVector` (.x (.location _outinstancetransform)) (.y (.location _outinstancetransform)) (select `bool` (>= _z _returnvalue_10) :`false` (`KismetMathLibrary.Lerp` _z _returnvalue_10 0.5) :`true` (`KismetMathLibrary.FInterpTo` _z 0.0 (`GameplayStatics.GetWorldDeltaSeconds`) 0.25))) (.rotation _outinstancetransform) (`self.top one scale`)))
            (bind _returnvalue_12 (`KismetMathLibrary.Clamp` (- _index _number_of_bars) 0 (- _number_of_bars 1)))
            (bind _output_2 (`|GetArrayItem` (`self.Tmp`) _returnvalue_12))
            (bind _transform_location (`KismetMathLibrary.BreakTransform` (`self.ローテーションから向きを取得` (`self.BaseTransform`) _returnvalue_12 (.z (.scale _output_2)))))
            (bind _returnvalue_13 (> (`KismetMathLibrary.VSize` _transform_location) (* (.z (.scale _output_2)) 100.0)))
            (bind _returnvalue_14 (> _index (- (`self.Number of bars`) 1)))
            (bind _output_3 (`|GetArrayItem` (`self.BaseTransform`) _returnvalue_8))
            (bind _returnvalue_15 (`KismetMathLibrary.MakeTransform` (`KismetMathLibrary.VLerp` (.location _outinstancetransform) (select `bool` _returnvalue_14 :`false` (.location _output) :`true` (`KismetMathLibrary.MakeVector` (+ (* (- (.x (.location _output)) (.x (.location _output_3))) -1.0) (.x (.location _output_3))) (+ (* (- (.y (.location _output)) (.y (.location _output_3))) -1.0) (.y (.location _output_3))) (* (.z (.location _output)) -1.0))) (- 1.0 (`self.smooth`))) (.rotation _output)))
            (`InstancedStaticMeshComponent.UpdateInstanceTransform` (`self.Ber`) _index (select `/Game/SoundVisualizerBP/Enum/BarMovement` (`self.Bar movement`) :`NewEnumerator0` _returnvalue_9 :`NewEnumerator1` (select `bool` _returnvalue_14 :`false` _returnvalue_9 :`true` (select `/Game/SoundVisualizerBP/Enum/BarType` (`self.Bar Type`) :`NewEnumerator0` _returnvalue_11 :`NewEnumerator1` (`KismetMathLibrary.MakeTransform` (select `bool` (select `/Game/SoundVisualizerBP/Enum/direction` (`self.direction`) :`NewEnumerator0` _returnvalue_13 :`NewEnumerator1` _returnvalue_13 :`NewEnumerator2` (> _z (* (.z (.scale _output_2)) 90.0))) :`false` (`KismetMathLibrary.VLerp` (.location _outinstancetransform) _transform_location 0.5) :`true` (`KismetMathLibrary.VInterpTo` (.location _outinstancetransform) (.location _output) (`GameplayStatics.GetWorldDeltaSeconds`) 0.25)) (.rotation _outinstancetransform) (1.0 1.0 0.5)) :`NewEnumerator3` _returnvalue_11 :`NewEnumerator5` _returnvalue_11)) :`NewEnumerator2` _returnvalue_15 :`NewEnumerator3` (`KismetMathLibrary.MakeTransform` (`KismetMathLibrary.VLerp` (.location _outinstancetransform) (.location _output) _returnvalue) (.rotation _output) (`KismetMathLibrary.MakeVector` (.x (.scale _outinstancetransform)) (.y (.scale _outinstancetransform)) (`KismetMathLibrary.Lerp` (.z (.scale _outinstancetransform)) (/ (.z (.location _output)) 100.0) _returnvalue))) :`NewEnumerator4` _returnvalue_15) false true false))))
      (set `self.stepheight` 0))))

(event `格納完了`
  (goto _label_2 :!via `Open`))

(event `Stop`
  (`AudioMixerBlueprintLibrary.StopAnalyzingOutput` null)
  (goto _label_2 :!via `Close`))

(fn `UserConstructionScript`
  (bind _number_of_bars (`self.Number of bars`))
  (bind _spline (`self.Spline`))
  (bind _bar_spacing (`self.Bar spacing`))
  (bind _x (`self.x`))
  (bind _bar_spacing_2 (`self.Bar spacing`))
  (bind _x_2 (`self.x`))
  (bind _radius (`self.radius`))
  (bind _number_of_bars_2 (`self.Number of bars`))
  (bind _number_of_bars_3 (`self.Number of bars`))
  (bind _spline_2 (`self.Spline`))
  (bind _bar_spacing_3 (`self.Bar spacing`))
  (bind _number_of_bars_4 (`self.Number of bars`))
  (bind _direction (`self.direction`))
  (bind _returnvalue (== (`self.Bar movement`) 5))
  (bind _returnvalue_2 (* (`self.y`) (`self.Bar spacing`)))
  (bind _returnvalue_3 (- (* (`self.Division number`) _number_of_bars_4) _number_of_bars_4))
  (bind _returnvalue_4 (+ (`self.radius`) (* _returnvalue_2 (select `/Game/SoundVisualizerBP/Enum/direction` _direction :`NewEnumerator0` -1.0 :`NewEnumerator1` 1.0 :!type "Float (single-precision)"))))
  (bind _returnvalue_5 (`KismetMathLibrary.Conv_IntToDouble` (`KismetMathLibrary.Round` (`KismetMathLibrary.Sqrt` (`KismetMathLibrary.Conv_IntToDouble` _number_of_bars)))))
  (bind _returnvalue_6 (/ (`KismetMathLibrary.Conv_IntToDouble` (`self.x`)) _returnvalue_5))
  (bind _returnvalue_7 (`KismetMathLibrary.Conv_IntToDouble` (`KismetMathLibrary.FFloor` _returnvalue_6)))
  (`SceneComponent.SetVisibility` (`self.Spline`) true false)
  (switch `/Game/SoundVisualizerBP/Enum/BarMovement` (`self.Bar movement`)
    (:`NewEnumerator0`
      _)
    (:`NewEnumerator1`
      (`StaticMeshComponent.SetStaticMesh` (`self.Ber`) "/Game/SoundVisualizerBP/Geometry/SM_BarOneSide.SM_BarOneSide"))
    (:`NewEnumerator2`
      _)
    (:`NewEnumerator3`
      _)
    (:`NewEnumerator4`
      _)
    (:`NewEnumerator5`
      _))
  (`KismetArrayLibrary.Array_Clear` (`self.Frequency`))
  (`KismetArrayLibrary.Array_Clear` (`self.BaseTransform`))
  (for _index (range 1 (+ _number_of_bars_2 1))
    (`KismetArrayLibrary.Array_Add` (`self.Frequency`) (`KismetMathLibrary.Conv_IntToDouble` (* _index (/ (`self.Frequency to analyze`) _number_of_bars_2))))
    (bind _angle_deg_ (`self.角度を計算` _index _number_of_bars_2))
    (bind _returnvalue_8 (* (/ (`KismetMathLibrary.Conv_IntToDouble` _index) (`KismetMathLibrary.Conv_IntToDouble` (`self.Number of bars`))) (`SplineComponent.GetSplineLength` _spline_2)))
    (bind _returnvalue_9 (select `/Game/SoundVisualizerBP/Enum/BarType` (`self.Bar Type`) :`NewEnumerator0` (`KismetMathLibrary.MakeTransform` (`KismetMathLibrary.MakeVector` 0.0 (* (- _index 1) (`self.Bar spacing`)))) :`NewEnumerator1` (`KismetMathLibrary.MakeTransform` (`KismetMathLibrary.MakeVector` (* (`KismetMathLibrary.DegCos` _angle_deg_) _radius) (* (`KismetMathLibrary.DegSin` _angle_deg_) _radius)) (`KismetMathLibrary.MakeRotator` 0.0 (select `/Game/SoundVisualizerBP/Enum/direction` (`self.direction`) :`NewEnumerator0` 90.0 :`NewEnumerator1` 270.0 :!type "Float (single-precision)") _angle_deg_)) :`NewEnumerator3` (`KismetMathLibrary.MakeTransform` (`KismetMathLibrary.MakeVector` (* (`self.x`) _bar_spacing_3) (* (`self.y`) _bar_spacing_3))) :`NewEnumerator5` (`KismetMathLibrary.MakeTransform` (* (`SplineComponent.GetLocationAtDistanceAlongSpline` _spline_2 _returnvalue_8 "Local") 50.0) (`SplineComponent.GetRotationAtDistanceAlongSpline` _spline_2 _returnvalue_8 "Local"))))
    (`InstancedStaticMeshComponent.AddInstance` (`self.Ber`) _returnvalue_9)
    (`KismetArrayLibrary.Array_Add` (`self.BaseTransform`) _returnvalue_9)
    ;[1 1 1] グリッド処理
    (`/Engine/EditorBlueprintResources/StandardMacros.IncrementInt` _x_2
      (:`  `
        (if (>= _x_2 (`KismetMathLibrary.Round` (`KismetMathLibrary.Sqrt` (`KismetMathLibrary.Conv_IntToDouble` _number_of_bars_2))))
          (`/Engine/EditorBlueprintResources/StandardMacros.IncrementInt` (`self.y`)
            (:`  `
              (set `self.x` 0)))))))
  (`/Engine/EditorBlueprintResources/StandardMacros.DoOnce` false
    (:`Completed`
      (if (or (`self.Top one Bers`) _returnvalue (== (`self.Bar movement`) 4))
        ;[1 1 1] 初期化
        (set `self.y` 1)
        (set `self.x` 0)
        (for _index_2 (range 1 (+ (select `bool` _returnvalue :`false` (`self.Number of bars`) :`true` (select `bool` (`self.Top one Bers`) :`false` _returnvalue_3 :`true` (+ _returnvalue_3 _number_of_bars_4))) 1))
          (bind _angle_deg__2 (`self.角度を計算` _index_2 _number_of_bars))
          (bind _returnvalue_10 (* (/ (`KismetMathLibrary.Conv_IntToDouble` (- _index_2 (* (`KismetMathLibrary.FFloor` (/ (`KismetMathLibrary.Conv_IntToDouble` _index_2) (`KismetMathLibrary.Conv_IntToDouble` _number_of_bars_3))) _number_of_bars_3))) (`KismetMathLibrary.Conv_IntToDouble` _number_of_bars_3)) (`SplineComponent.GetSplineLength` _spline)))
          (bind (_returnvalue_x _returnvalue_y _returnvalue_z) (`KismetMathLibrary.BreakVector` (`SplineComponent.GetLocationAtDistanceAlongSpline` _spline _returnvalue_10 "Local")))
          (`InstancedStaticMeshComponent.AddInstance` (`self.Ber`) (select `/Game/SoundVisualizerBP/Enum/BarType` (`self.Bar Type`) :`NewEnumerator0` (`KismetMathLibrary.MakeTransform` (`KismetMathLibrary.MakeVector` 0.0 (* (`self.x`) _bar_spacing_2) (* (`self.y`) _bar_spacing_2))) :`NewEnumerator1` (`KismetMathLibrary.MakeTransform` (`KismetMathLibrary.MakeVector` (* (`KismetMathLibrary.DegCos` _angle_deg__2) _returnvalue_4) (* (`KismetMathLibrary.DegSin` _angle_deg__2) _returnvalue_4) (select `/Game/SoundVisualizerBP/Enum/direction` _direction :`NewEnumerator2` _returnvalue_2)) (`KismetMathLibrary.MakeRotator` 0.0 (select `/Game/SoundVisualizerBP/Enum/direction` _direction :`NewEnumerator0` 90.0 :`NewEnumerator1` 270.0 :!type "Float (single-precision)") _angle_deg__2)) :`NewEnumerator3` (`KismetMathLibrary.MakeTransform` (`KismetMathLibrary.MakeVector` (* (- _returnvalue_6 _returnvalue_7) _returnvalue_5 _bar_spacing) (* _returnvalue_7 _bar_spacing) (* (`self.y`) _bar_spacing))) :`NewEnumerator5` (`KismetMathLibrary.MakeTransform` (* (`KismetMathLibrary.MakeVector` _returnvalue_x _returnvalue_y (+ _returnvalue_z (/ (* (`self.y`) (`self.Bar spacing`)) 25.0))) 50.0) (`SplineComponent.GetRotationAtDistanceAlongSpline` _spline _returnvalue_10 "Local"))))
          (`/Engine/EditorBlueprintResources/StandardMacros.IncrementInt` _x
            (:`  `
              (if (>= _x (`self.Number of bars`))
                (`/Engine/EditorBlueprintResources/StandardMacros.IncrementInt` (`self.y`)
                  (:`  `
                    (set `self.x` 0)))))))))))

(fn `ローテーションから向きを取得`
  (params (Transforms :type "Array of Transform Structure") (Index :type Integer) (Strength :type "Float (double-precision)"))
  (returns (Transform :type "Transform Structure"))
  (bind _returnvalue (* 100 Strength))
  (bind _output (`|GetArrayItem` Transforms Index))
  (bind (_output_location _output_rotation _output_scale) (`KismetMathLibrary.BreakTransform` (`|GetArrayItem` Transforms Index)))
  (bind _angle_deg_ (`self.角度を計算` Index (`KismetArrayLibrary.Array_Length` Transforms)))
  (bind _returnvalue_2 (`KismetMathLibrary.DegSin` (* (.pitch (.rotation _output)) -1.0)))
  (return (`KismetMathLibrary.MakeTransform` (`KismetMathLibrary.MakeVector` (+ (.x (.location _output)) (* _returnvalue (`KismetMathLibrary.DegCos` _angle_deg_) _returnvalue_2)) (+ (.y (.location _output)) (* _returnvalue (`KismetMathLibrary.DegSin` _angle_deg_) _returnvalue_2)) (* (`KismetMathLibrary.DegCos` (.pitch (.rotation _output))) _returnvalue)) _output_rotation _output_scale)))

(fn `角度を計算`
  (params (Index :type Integer) (Length :type Integer))
  (returns (`Angle(Deg)` :type "Float (double-precision)"))
  (return (* (/ (`KismetMathLibrary.Conv_IntToDouble` Index) (`KismetMathLibrary.Conv_IntToDouble` Length)) 360.0)))