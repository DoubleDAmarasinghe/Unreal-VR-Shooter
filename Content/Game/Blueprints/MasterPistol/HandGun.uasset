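; VR handgun actor that can be grabbed by either motion controller and fired from that hand.
; Grab checks the grip sphere, disables physics and attaches the gun to the hand's holder socket; Release detaches it and restores physics.
; Per-hand fire events consume ammo, play sound and muzzle flash, and spawn a muzzle projectile only when a line trace hits.
; Empty shots click; recoil nodes are unconnected.
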(event `self.ReceiveBeginPlay`
  ;[1 1 1] Create References
  (bind _returnvalue (`GameplayStatics.GetActorOfClass` "/Game/Game/Blueprints/Pawns/VR_Pawn.VR_Pawn_C"))
  (set `self.VRPawn` _returnvalue))

(event `HandGunFireRight`
  (bind _staticmesh (`self.StaticMesh`))
  (bind _staticmesh_2 (`self.StaticMesh`))
  (bind _returnvalue (`SceneComponent.GetSocketLocation` _staticmesh_2 "MuzzleLocation"))
  ;[1 1 1] HandGun Fire Right Hand
  (if (and (`self.CanFireRight`) (> (`self.AmmoCount`) 0) (== (`/Game/Game/Blueprints/Pawns/VR_Pawn.RightGrabActor` (`self.VRPawn`)) self))
    (set `self.AmmoCount` (- (`self.AmmoCount`) 1))
    (bind _returnvalue_2 (`GameplayStatics.CreateSound2D` "/Game/Game/Sounds/SHOT2.SHOT2" 1.0 1.0 0.0 null))
    (`AudioComponent.Play` _returnvalue_2 0.0)
    (`GameplayStatics.SpawnEmitterAtLocation` "/Game/MilitaryWeapDark/FX/P_AssaultRifle_MuzzleFlash.P_AssaultRifle_MuzzleFlash" (`SceneComponent.GetSocketLocation` _staticmesh "MuzzleLocation") (`SceneComponent.GetSocketRotation` _staticmesh "MuzzleLocation") (0.5 0.5 0.5))
    (bind (_outhit _returnvalue_3) (`KismetSystemLibrary.LineTraceSingle` _returnvalue (+ _returnvalue (* (`KismetMathLibrary.GetRightVector` (`SceneComponent.K2_GetComponentRotation` _staticmesh_2)) 500000.0)) "TraceTypeQuery1"))
    (if _returnvalue_3
      (bind (_bblockinghit _binitialoverlap _time _distance _location _impactpoint _normal _impactnormal _physmat _hitactor _hitcomponent _hitbonename _hititem _elementindex _faceindex _tracestart _traceend) (`GameplayStatics.BreakHitResult` _outhit))
      (`|SpawnActorFromClass` "/Game/VRTemplate/Blueprints/Projectile.Projectile_C" (`KismetMathLibrary.MakeTransform` _returnvalue (`KismetMathLibrary.FindLookAtRotation` _location _traceend)) "AlwaysSpawn" "OverrideRootScale" null null))
    (else
      ;;[1 1 1] If Doesn't Have Ammo
      (if (and (`self.CanFireRight`) (== (`self.AmmoCount`) 0))
        (bind _returnvalue_4 (`GameplayStatics.CreateSound2D` "/Game/Game/Sounds/EmptyRound.EmptyRound" 1.0 1.0 0.0 null))
        (`AudioComponent.Play` _returnvalue_4 0.0)))))

(event `/Game/Game/Interfaces/Pickup.Grab`
  (params (MotionController :type "MotionControllerComponent Object Reference"))
  (bind _grip (`self.Grip`))
  ;[0.02745 0.3608 1] Interface Grab Action
  (if (<= (`KismetMathLibrary.Vector_Distance` (`SceneComponent.K2_GetComponentLocation` MotionController) (`SceneComponent.K2_GetComponentLocation` _grip)) (`SphereComponent.SphereRadius` _grip))
    (bind _output_get (set `self.MainGrip` MotionController))
    (`PrimitiveComponent.SetSimulatePhysics` (`self.StaticMesh`) false)
    (`|ExecutionSequence`
      (:`then_0`
        (if (== _output_get (`/Game/Game/Blueprints/Pawns/VR_Pawn.MotionControllerRight` (`self.VRPawn`)))
          (`self.K2_AttachToComponent` (`/Game/Game/Blueprints/Pawns/VR_Pawn.HandRight` (`self.VRPawn`)) "RightHandGunHolder" "SnapToTarget" "SnapToTarget" "KeepRelative")
          (set `self.CanFireRight` true)))
      (:`then_1`
        (if (== _output_get (`/Game/Game/Blueprints/Pawns/VR_Pawn.MotionControllerLeft` (`self.VRPawn`)))
          (`self.K2_AttachToComponent` (`/Game/Game/Blueprints/Pawns/VR_Pawn.HandLeft` (`self.VRPawn`)) "LeftHandGunHolder" "SnapToTarget" "SnapToTarget" "KeepRelative")
          (set `self.CanFireLeft` true))))))

(event `/Game/Game/Interfaces/Pickup.Release`
  (params (Motioncontroller :type "MotionControllerComponent Object Reference"))
  ;[0.02745 0.3608 1] Interface Release Acrion
  (if (== Motioncontroller (`self.MainGrip`))
    (`PrimitiveComponent.SetSimulatePhysics` (`self.StaticMesh`) true)
    (set `self.MainGrip` null)
    (`self.K2_DetachFromActor` "KeepWorld" "KeepWorld" "KeepWorld")
    (set `self.CanFireLeft` false)
    (set `self.CanFireRight` false)))

(event `HandGunFireLeft`
  (bind _staticmesh (`self.StaticMesh`))
  (bind _staticmesh_2 (`self.StaticMesh`))
  (bind _returnvalue (`SceneComponent.GetSocketLocation` _staticmesh_2 "MuzzleLocation"))
  ;[1 1 1] HandGun Fire Right Hand
  (if (and (`self.CanFireLeft`) (> (`self.AmmoCount`) 0) (== (`/Game/Game/Blueprints/Pawns/VR_Pawn.LeftGrabactor` (`self.VRPawn`)) self))
    (set `self.AmmoCount` (- (`self.AmmoCount`) 1))
    (bind _returnvalue_2 (`GameplayStatics.CreateSound2D` "/Game/Game/Sounds/SHOT2.SHOT2" 1.0 1.0 0.0 null))
    (`AudioComponent.Play` _returnvalue_2 0.0)
    (`GameplayStatics.SpawnEmitterAtLocation` "/Game/MilitaryWeapDark/FX/P_AssaultRifle_MuzzleFlash.P_AssaultRifle_MuzzleFlash" (`SceneComponent.GetSocketLocation` _staticmesh "MuzzleLocation") (`SceneComponent.GetSocketRotation` _staticmesh "MuzzleLocation") (0.5 0.5 0.5))
    (bind (_outhit _returnvalue_3) (`KismetSystemLibrary.LineTraceSingle` _returnvalue (+ _returnvalue (* (`KismetMathLibrary.GetRightVector` (`SceneComponent.K2_GetComponentRotation` _staticmesh_2)) 500000.0)) "TraceTypeQuery1"))
    (if _returnvalue_3
      (bind (_bblockinghit _binitialoverlap _time _distance _location _impactpoint _normal _impactnormal _physmat _hitactor _hitcomponent _hitbonename _hititem _elementindex _faceindex _tracestart _traceend) (`GameplayStatics.BreakHitResult` _outhit))
      (`|SpawnActorFromClass` "/Game/VRTemplate/Blueprints/Projectile.Projectile_C" (`KismetMathLibrary.MakeTransform` _returnvalue (`KismetMathLibrary.FindLookAtRotation` _location _traceend)) "AlwaysSpawn" "OverrideRootScale" null null)
      (`KismetSystemLibrary.Delay` 0.1))
    (else
      ;;[1 1 1] If Doesn't Have Ammo
      (if (and (`self.CanFireLeft`) (== (`self.AmmoCount`) 0))
        (bind _returnvalue_4 (`GameplayStatics.CreateSound2D` "/Game/Game/Sounds/EmptyRound.EmptyRound" 1.0 1.0 0.0 null))
        (`AudioComponent.Play` _returnvalue_4 0.0)))))

(fn `UserConstructionScript`)