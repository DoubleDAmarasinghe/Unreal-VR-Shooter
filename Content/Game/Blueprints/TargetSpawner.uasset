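; TargetSpawner Blueprint that spawns shooting or scoring targets and awards points through a SpawnTargets custom event.
; After a short delay, the event increases Points and plays a 2D spawn sound.
; It then spawns a Target actor at the transform of a randomly chosen entry from ten TargetPoint references.
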(event `SpawnTargets`
  ;[1 1 1] Target Spawning Event
  (`KismetSystemLibrary.Delay` 0.5)
  (set `self.Points` (+ (`self.Points`) 5.0))
  (`GameplayStatics.PlaySound2D` "/Game/Game/Sounds/252083__pepingrillin__spawn.252083__pepingrillin__spawn" 1.0 1.0 0.0 null null)
  (`|SpawnActorFromClass` "/Game/Game/Blueprints/Target.Target_C" (`self.GetTransform` (`|GetArrayItem` (`|MakeArray` (`self.targetPoint1`) (`self.targetPoint2`) (`self.targetPoint3`) (`self.targetPoint4`) (`self.targetPoint5`) (`self.targetPoint6`) (`self.targetPoint7`) (`self.targetPoint8`) (`self.targetPoint9`) (`self.targetPoint10`)) (`KismetMathLibrary.RandomIntegerInRange` 0 9))) "Undefined" "OverrideRootScale" null null))

(fn `UserConstructionScript`)