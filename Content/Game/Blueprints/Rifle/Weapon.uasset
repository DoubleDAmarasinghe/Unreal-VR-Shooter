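; Two-handed VR rifle actor that responds to interface Grab and Release events from motion controllers.
; Grab matches the controller to one of two grip spheres by distance; the first grip also attaches to the character's right-hand socket.
; With both grips held, Tick aims the weapon along the line between controllers, remapping axes and using the first controller's roll.
; Releasing the first grip detaches it; releasing only the second resets its relative transform from a mesh socket.
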(event `self.ReceiveTick`
  (params (DeltaSeconds :type "Float (single-precision)"))
  (bind _first_grip_controller (`self.first Grip Controller`))
  (bind _returnvalue_roll (`KismetMathLibrary.BreakRotator` (`SceneComponent.K2_GetComponentRotation` _first_grip_controller)))
  (bind (_returnvalue_roll_2 _returnvalue_pitch _returnvalue_yaw) (`KismetMathLibrary.BreakRotator` (`KismetMathLibrary.ComposeRotators` (`KismetMathLibrary.FindLookAtRotation` (`SceneComponent.K2_GetComponentLocation` _first_grip_controller) (`SceneComponent.K2_GetComponentLocation` (`self.SecondGripController`))) (struct :`Yaw` -90.0))))
  (if (and (`KismetSystemLibrary.IsValid` (`self.first Grip Controller`)) (`KismetSystemLibrary.IsValid` (`self.SecondGripController`)))
    (`self.K2_SetActorRotation` (`KismetMathLibrary.MakeRotator` (* _returnvalue_pitch -1.0) _returnvalue_roll _returnvalue_yaw))))

(event `self.ReceiveBeginPlay`
  (bind _returnvalue (`GameplayStatics.GetActorOfClass` "/Game/VRTemplate/Blueprints/NewVR/NewVRCharacter.NewVRCharacter_C"))
  (set `self.VRPlayerRef` _returnvalue))

(event `/Game/Game/Interfaces/Pickup.Grab`
  (params (MotionController :type "MotionControllerComponent Object Reference"))
  (bind _grip1 (`self.Grip1`))
  (bind _grip2 (`self.Grip2`))
  ;[0.02745 0.3608 1] Interface Grab Acrion
  (if (<= (`KismetMathLibrary.Vector_Distance` (`SceneComponent.K2_GetComponentLocation` MotionController) (`SceneComponent.K2_GetComponentLocation` _grip1)) (`SphereComponent.SphereRadius` _grip1))
    (set `self.first Grip Controller` MotionController)
    (`self.K2_AttachToComponent` (`/Game/VRTemplate/Blueprints/NewVR/NewVRCharacter.SkeletalMeshRight` (`self.VRPlayerRef`)) "RightHolder" "SnapToTarget" "SnapToTarget" "KeepRelative")
    (elif (<= (`KismetMathLibrary.Vector_Distance` (`SceneComponent.K2_GetComponentLocation` MotionController) (`SceneComponent.K2_GetComponentLocation` _grip2)) (`SphereComponent.SphereRadius` _grip2))
      (set `self.SecondGripController` MotionController))))

(event `/Game/Game/Interfaces/Pickup.Release`
  (params (Motioncontroller :type "MotionControllerComponent Object Reference"))
  ;[0.02745 0.3608 1] Interface Release Action
  (`|ExecutionSequence`
    (:`then_0`
      (if (== Motioncontroller (`self.first Grip Controller`))
        (set `self.first Grip Controller` null)
        (set `self.SecondGripController` null)
        (`self.K2_DetachFromActor` "KeepWorld" "KeepWorld" "KeepWorld")))
    (:`then_1`
      (if (== Motioncontroller (`self.SecondGripController`))
        (set `self.SecondGripController` null)
        (`self.first Grip Controller`
          (:`then`
            (`self.K2_SetActorRelativeTransform` (`SceneComponent.GetSocketTransform` (`self.WeaponMesh`) "SecondGrab" "RTS_Actor")))
          (:`else`
            (`self.K2_DetachFromActor` "KeepWorld" "KeepWorld" "KeepWorld")))))))

(fn `UserConstructionScript`)